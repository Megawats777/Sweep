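; BP_PlayerCharacter is the first-person player character for a score attack game, handling movement, look, shooting and pausing.
; Axis inputs drive actor-relative movement and sensitivity-scaled controller look, with look gated by CanLook.
; Fire spawns a BP_Projectile at the camera's location and rotation.
; Pause calls the score attack game mode, cached on BeginPlay, only while the game is active and not already paused.
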(event `self.ReceiveBeginPlay`
  (bind _asbp_score_attack_game_mode (cast `/Game/Blueprints/BP_ScoreAttackGameMode` (`GameplayStatics.GetGameMode`)))
  (set `self.ScoreAttackGameModeRef` _asbp_score_attack_game_mode))

(event `InputAxis|ForwardBackwardsMovement`
  (params (AxisValue :type "Float (single-precision)"))
  ;[1 1 1] Forward / Backwards Movement
  (`self.AddMovementInput` (`KismetMathLibrary.GetForwardVector` (`self.K2_GetActorRotation`)) AxisValue))

(event `InputAxis|RightLeftMovement`
  (params (AxisValue :type "Float (single-precision)"))
  ;[1 1 1] Right / Left Movement
  (`self.AddMovementInput` (`KismetMathLibrary.GetRightVector` (`self.K2_GetActorRotation`)) AxisValue))

(event `InputAxis|VerticalLook`
  (params (AxisValue :type "Float (single-precision)"))
  ;[1 1 1] Vertical Look
  (if (`self.CanLook`)
    (`self.AddControllerPitchInput` (* AxisValue (`self.LookSensitivity`)))))

(event `InputAxis|HorizontalLook`
  (params (AxisValue :type "Float (single-precision)"))
  ;[1 1 1] Horizontal Look
  (if (`self.CanLook`)
    (`self.AddControllerYawInput` (* AxisValue (`self.LookSensitivity`)))))

(event `InputAction|Fire`
  (params (Key :type "Key Structure" :default "AnyKey"))
  (bind _camera (`self.Camera`))
  ;[1 1 1] Fire a projectile
  (:`Pressed`
    (`|SpawnActorFromClass` "/Game/Blueprints/BP_Projectile.BP_Projectile_C" (`KismetMathLibrary.MakeTransform` (`SceneComponent.K2_GetComponentLocation` _camera) (`SceneComponent.K2_GetComponentRotation` _camera) (1.0 1.0 1.0)) "Undefined" "OverrideRootScale")))

(event `InputAction|Pause`
  (params (Key :type "Key Structure" :default "AnyKey"))
  (bind _currentgamestate (`/Game/Blueprints/BP_ScoreAttackGameMode.CurrentGameState` (`self.ScoreAttackGameModeRef`)))
  ;[1 1 1] Pause the game
  (:`Pressed`
    (if (and (`/Game/Blueprints/BPFL_GameStateCheckers.isGameActive` _currentgamestate) (== (`/Game/Blueprints/BPFL_GameStateCheckers.isGamePaused` _currentgamestate) false))
      (`/Game/Blueprints/BP_ScoreAttackGameMode.PauseGame` (`self.ScoreAttackGameModeRef`)))))

(fn `UserConstructionScript`)