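; Score attack target actor that awards its score value and adds to the player's streak when destroyed during an active game.
; Destruction only hides it and disables collision, so RespawnTarget can restore the same actor.
; SetPotentialPositions stores locations from linked PotentialPositionObjects, though no movement happens here.
; The construction script draws debug lines to those objects to visualise the links.
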(event `self.ReceiveBeginPlay`
  ;[1 1 1] Get a reference to the score attack game mode
  (bind _asbp_score_attack_game_mode (cast `/Game/Blueprints/BP_ScoreAttackGameMode` (`GameplayStatics.GetGameMode`)))
  (set `self.ScoreAttackGameModeRef` _asbp_score_attack_game_mode))

(event `RespawnTarget`
  ;[1 1 1] Respawn this target
  (`self.SetActorEnableCollision` true)
  (`SceneComponent.SetVisibility` (`self.Root`) true true))

(event `DestroyTarget`
  ;[1 1 1] Destroy this target
  (if (`|EnumEquality` (`/Game/Blueprints/BP_ScoreAttackGameMode.CurrentGameState` (`self.ScoreAttackGameModeRef`)) "NewEnumerator1")
    (`/Game/Blueprints/BP_ScoreAttackGameMode.IncreasePlayerScore` (`self.ScoreAttackGameModeRef`) (`self.ScoreValue`))
    (`self.SetActorEnableCollision` false)
    (`SceneComponent.SetVisibility` (`self.Root`) false true)
    (`/Game/Blueprints/BP_ScoreAttackGameMode.IncreaseCurrentStreak` (`self.ScoreAttackGameModeRef`) 1)))

(event `SetPotentialPositions`
  (`KismetArrayLibrary.Array_Set` (`self.PotentialPositions`) 0 (`self.K2_GetActorLocation`) true)
  (for (_array_element _array_index) (`self.PotentialPositionObjects`)
    (`KismetArrayLibrary.Array_Set` (`self.PotentialPositions`) _array_index (`self.K2_GetActorLocation` _array_element) true)))

(fn `UserConstructionScript`
  (`KismetSystemLibrary.FlushPersistentDebugLines`)
  (for _array_element (`self.PotentialPositionObjects`)
    (if (`KismetSystemLibrary.IsValid` _array_element)
      (`KismetSystemLibrary.DrawDebugLine` (`self.K2_GetActorLocation`) (`self.K2_GetActorLocation` _array_element) (struct :`R` 0.835 :`B` 0.016106 :`A` 1.0) 99.0 5.0))))