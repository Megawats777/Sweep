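; BP_Projectile is a projectile for a score attack mode that destroys BP_Target actors on impact.
; On BeginPlay it applies its desired scale and caches the BP_ScoreAttackGameMode.
; Each Tick it moves along its forward vector by Speed with a swept SetActorLocation, without delta-time scaling.
; A hit either destroys the target or resets the game mode's score multiplier and current streak, then the projectile destroys itself.
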(event `self.ReceiveBeginPlay`
  ;[1 1 1] Set the size of this projectile based on the desired scale value
  (`self.SetActorScale3D` (`self.DesiredScale`))
  (bind _asbp_score_attack_game_mode (cast `/Game/Blueprints/BP_ScoreAttackGameMode` (`GameplayStatics.GetGameMode`)))
  (set `self.ScoreAttackGameModeRef` _asbp_score_attack_game_mode))

(event `self.ReceiveTick`
  (params (DeltaSeconds :type "Float (single-precision)"))
  ;[1 1 1] Move forward every frame
  (`self.MoveForward`))

(event `MoveForward`
  ;[1 1 1] Move this projectile forward
  (`self.K2_SetActorLocation` (+ (`self.K2_GetActorLocation`) (* (`KismetMathLibrary.GetForwardVector` (`self.K2_GetActorRotation`)) (`self.Speed`))) true))

(event `self.ReceiveHit`
  (params (MyComp :type "PrimitiveComponent Object Reference") (Other :type "Actor Object Reference") (OtherComp :type "PrimitiveComponent Object Reference") (bSelfMoved :type Boolean) (HitLocation :type "Vector Structure") (HitNormal :type "Vector Structure") (NormalImpulse :type "Vector Structure") (Hit :type "HitResult Structure (by ref)"))
  ;[1 1 1] When this projectile is hit
  (bind _asbp_target (cast `/Game/Blueprints/BP_Target` Other) ; If the object hit is a target
    (:`then`
      (`/Game/Blueprints/BP_Target.DestroyTarget` _asbp_target) ; Destroy the target
      (`self.DestroyProjectile`))
    (:`CastFailed`
      ;;[1 0.9763 0.4799] If the object hit is not a target reset the score multiplier and reset the player's current streak
      (`/Game/Blueprints/BP_ScoreAttackGameMode.ResetScoreMultiplier` (`self.ScoreAttackGameModeRef`))
      (`/Game/Blueprints/BP_ScoreAttackGameMode.ResetCurrentStreak` (`self.ScoreAttackGameModeRef`))
      (`self.DestroyProjectile`))))

(event `DestroyProjectile`
  ;[1 1 1] Destroy this projectile
  (`self.K2_DestroyActor`))

(fn `UserConstructionScript`)