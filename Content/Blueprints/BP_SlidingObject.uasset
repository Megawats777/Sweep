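; BP_SlidingObject is a configurable mesh that slides to a marker location when the player enters its trigger box.
; The SlidingMovement timeline lerps the mesh from the actor's start location to the cached marker position at an adjustable speed.
; On exit, the timeline can optionally reverse to return the mesh.
; The construction script applies the chosen mesh, trigger size and placement, and destination marker location for per-instance setup.
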(event `self.ReceiveBeginPlay`
  (bind _asbp_player_character (cast `/Game/Blueprints/BP_PlayerCharacter` (`GameplayStatics.GetPlayerCharacter` 0)))
  (set `self.PlayerCharacter` _asbp_player_character)
  (set `self.StartingLocation` (`self.K2_GetActorLocation`))
  (set `self.SlideDestination` (`SceneComponent.K2_GetComponentLocation` (`self.SlideDestinationMarker`)))
  ;[1 1 1] Set the movement speed of the sliding movement
  (`TimelineComponent.SetPlayRate` (`self.SlidingMovement`) (`self.SlidingSpeed`)))

(event `self.TriggerBox.OnComponentBeginOverlap`
  (params (OverlappedComponent :type "PrimitiveComponent Object Reference") (OtherActor :type "Actor Object Reference") (OtherComp :type "PrimitiveComponent Object Reference") (OtherBodyIndex :type Integer) (bFromSweep :type Boolean) (SweepResult :type "HitResult Structure (by ref)"))
  ;[1 1 1] When the trigger box is overlaped
  (if (== OtherActor (`self.PlayerCharacter`))
    (`self.BlendToSlideDestination`)))

(event `self.TriggerBox.OnComponentEndOverlap`
  (params (OverlappedComponent :type "PrimitiveComponent Object Reference") (OtherActor :type "Actor Object Reference") (OtherComp :type "PrimitiveComponent Object Reference") (OtherBodyIndex :type Integer))
  ;[1 1 1] When the trigger box is no longer overlaped
  (if (== OtherActor (`self.PlayerCharacter`))
    (if (`self.RevertsToOriginalPosition`)
      (`self.BlendToStartingLocation`))))

(event `BlendToSlideDestination`
  ;[1 1 1] Sliding movement
  (bind (_direction _movementcurve) (`Timeline|SlidingMovement` :!label _label)
    (:`Update`
      (`SceneComponent.K2_SetWorldLocation` (`self.SlidingMesh`) (`KismetMathLibrary.VLerp` (`self.StartingLocation`) (`self.SlideDestination`) _movementcurve) false false))))

(event `BlendToStartingLocation`
  (goto _label :!via `Reverse`))

(fn `UserConstructionScript`
  ;[1 1 1] Set the size and location of the trigger box
  (`SceneComponent.SetRelativeScale3D` (`self.TriggerBox`) (`self.TriggerBoxSize`))
  (`SceneComponent.K2_SetRelativeLocation` (`self.TriggerBox`) (`self.TriggerBoxLocation`) false false)
  ;[1 1 1] Set the location of the slide destination marker
  (`SceneComponent.K2_SetRelativeLocation` (`self.SlideDestinationMarker`) (`self.SlideDestinationMarkerLocation`) false false)
  ;[1 1 1] Set the chosen displayed sliding mesh
  (`StaticMeshComponent.SetStaticMesh` (`self.SlidingMesh`) (`self.ChosenSlidingMesh`)))