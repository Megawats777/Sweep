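; BP_StartPortal is a portal actor that starts a score attack run when the player enters it.
; On BeginPlay it caches the score attack game mode.
; When the player character overlaps the portal mesh and the game state is starting, it calls StartGame on that game mode.
; The construction script applies the configurable portal mesh scale and display text position.
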(event `self.ReceiveBeginPlay`
  (bind _asbp_score_attack_game_mode (cast `/Game/Blueprints/BP_ScoreAttackGameMode` (`GameplayStatics.GetGameMode`)))
  (set `self.ScoreAttackGameModeRef` _asbp_score_attack_game_mode))

(event `self.PortalMesh.OnComponentBeginOverlap`
  (params (OverlappedComponent :type "PrimitiveComponent Object Reference") (OtherActor :type "Actor Object Reference") (OtherComp :type "PrimitiveComponent Object Reference") (OtherBodyIndex :type Integer) (bFromSweep :type Boolean) (SweepResult :type "HitResult Structure (by ref)"))
  ;[1 1 1] When the portal mesh is overlaped
  (cast `/Game/Blueprints/BP_PlayerCharacter` OtherActor) ; If the overlaping object is the player
  (if (`/Game/Blueprints/BPFL_GameStateCheckers.isGameStarting` (`/Game/Blueprints/BP_ScoreAttackGameMode.CurrentGameState` (`self.ScoreAttackGameModeRef`)))
    (`/Game/Blueprints/BP_ScoreAttackGameMode.StartGame` (`self.ScoreAttackGameModeRef`))))

(fn `UserConstructionScript`
  ;[1 1 1] Set the size of the portal mesh
  (`SceneComponent.SetWorldScale3D` (`self.PortalMesh`) (`self.PortalSize`))
  ;[1 1 1] Set the location of the display text
  (`SceneComponent.K2_SetRelativeLocation` (`self.DisplayText`) (`self.DisplayTextLocation`) false false))