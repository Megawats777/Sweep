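; BP_Teleporter_FinishLine is a child teleporter that acts as the finish line of a score attack run.
; It caches the BP_ScoreAttackGameMode on BeginPlay.
; On TeleportPlayer it respawns every BP_Target in the level, then has the game mode increase the score multiplier and end the current run before the parent performs its teleport logic.
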(event `self.ReceiveBeginPlay`
  (`parent.ReceiveBeginPlay`)
  (bind _asbp_score_attack_game_mode (cast `/Game/Blueprints/BP_ScoreAttackGameMode` (`GameplayStatics.GetGameMode`)))
  (set `self.ScoreAttackGameModeRef` _asbp_score_attack_game_mode))

(event `self.TeleportPlayer`
  ;[1 1 1] Teleport player event
  ;;[1 0.96 0.5289] Get all targets and respawn them
  (bind _outactors (`GameplayStatics.GetAllActorsOfClass` "/Game/Blueprints/BP_Target.BP_Target_C"))
  (for _array_element _outactors
    (`/Game/Blueprints/BP_Target.RespawnTarget` _array_element))
  (`/Game/Blueprints/BP_ScoreAttackGameMode.IncreaseScoreMultiplier` (`self.ScoreAttackGameModeRef`) 1)
  (`/Game/Blueprints/BP_ScoreAttackGameMode.EndCurrentRun` (`self.ScoreAttackGameModeRef`))
  (`parent.TeleportPlayer`))

(fn `UserConstructionScript`
  (`parent.UserConstructionScript`))