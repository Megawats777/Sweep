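; BP_LevelConstructionTile is a level-building tile actor that assembles itself in its Construction Script, with no active runtime logic.
; RoofHeight multiplies the roof's offset Z position to place it.
; LeftWallHeight drives a loop adding wall mesh components, tracked in LeftWallsSpawned.
; Segments after the first derive Z from the array entry at the current one-based loop index, intending a vertical stack.
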(fn `UserConstructionScript`
  (locals (SpawnedLeftWall :type "StaticMeshComponent Object Reference") (LeftWallSpawnLoopIndex :type Integer))
  (bind (_relativelocation_x _relativelocation_y _relativelocation_z) (`KismetMathLibrary.BreakVector` (`SceneComponent.RelativeLocation` (`self.Roof`))))
  (bind (_relativelocation_x_2 _relativelocation_y_2 _relativelocation_z_2) (`KismetMathLibrary.BreakVector` (`SceneComponent.RelativeLocation` (`KismetArrayLibrary.Array_Get` (`self.LeftWallsSpawned`) (`local.LeftWallSpawnLoopIndex`)))))
  ;[1 1 1] Set the height of the roof
  (`SceneComponent.K2_SetRelativeLocation` (`self.Roof`) (`KismetMathLibrary.MakeVector` 0.0 0.0 (* (`self.RoofHeight`) (+ _relativelocation_z 20.0))) false false)
  (if (> (`self.LeftWallHeight`) 0)
    (for _index (range 1 (+ (`self.LeftWallHeight`) 1))
      (set `local.LeftWallSpawnLoopIndex` _index)
      (if (> _index 1)
        (bind _returnvalue (`AddComponent|NODE_AddStaticMeshComponent-0` :`RelativeTransform` (`KismetMathLibrary.MakeTransform` (`KismetMathLibrary.MakeVector` 0.0 10.0 (+ _relativelocation_z_2 400.0)))))
        (set `local.SpawnedLeftWall` _returnvalue)
        (`KismetArrayLibrary.Array_Add` (`self.LeftWallsSpawned`) (`local.SpawnedLeftWall`))
        (else
          (bind _returnvalue_2 (`AddComponent|NODE_AddStaticMeshComponent-1` :`RelativeTransform` (`KismetMathLibrary.MakeTransform` (0.0 10.0 0.0))))
          (set `local.SpawnedLeftWall` _returnvalue_2)
          (`KismetArrayLibrary.Array_Add` (`self.LeftWallsSpawned`) (`local.SpawnedLeftWall`)))))
    (else
      (`KismetArrayLibrary.Array_Clear` (`self.LeftWallsSpawned`)))))