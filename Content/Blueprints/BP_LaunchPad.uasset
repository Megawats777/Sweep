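; BP_LaunchPad is a launch pad that flings the player character when they step onto it.
; It caches the player on BeginPlay, and when that player overlaps TriggerBox it overrides their velocity with a launch built from the pad's forward and up vectors, each scaled by its own force.
; The construction script scales PadMesh in X and Y from LaunchPadSize, keeping its existing height.
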(event `self.ReceiveBeginPlay`
  (bind _asbp_player_character (cast `/Game/Blueprints/BP_PlayerCharacter` (`GameplayStatics.GetPlayerCharacter` 0)))
  (set `self.PlayerCharacter` _asbp_player_character))

(event `self.TriggerBox.OnComponentBeginOverlap`
  (params (OverlappedComponent :type "PrimitiveComponent Object Reference") (OtherActor :type "Actor Object Reference") (OtherComp :type "PrimitiveComponent Object Reference") (OtherBodyIndex :type Integer) (bFromSweep :type Boolean) (SweepResult :type "HitResult Structure (by ref)"))
  (bind _returnvalue (`self.K2_GetActorRotation`))
  (if (== OtherActor (`self.PlayerCharacter`))
    ;[1 1 1] Launch the player character
    (`Character.LaunchCharacter` (`self.PlayerCharacter`) (+ (* (`KismetMathLibrary.GetForwardVector` _returnvalue) (`self.ForwardLaunchForce`)) (* (`KismetMathLibrary.GetUpVector` _returnvalue) (`self.UpLaunchForce`))) true true)))

(fn `UserConstructionScript`
  (bind _padmesh (`self.PadMesh`))
  (bind (_launchpadsize_x _launchpadsize_y) (`KismetMathLibrary.BreakVector` (`self.LaunchPadSize`)))
  (bind (_relativescale3d_x _relativescale3d_y _relativescale3d_z) (`KismetMathLibrary.BreakVector` (`SceneComponent.RelativeScale3D` _padmesh)))
  (`SceneComponent.SetRelativeScale3D` _padmesh (`KismetMathLibrary.MakeVector` _launchpadsize_x _launchpadsize_y _relativescale3d_z)))