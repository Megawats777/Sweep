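; BP_GameHUDManager creates and holds the game's HUD widgets for the start, main game, game over and pause screens.
; On BeginPlay it creates each widget for player controller 0 and stores it in its own variable.
; Only the start screen is shown immediately, through its ShowHUD call; the other three are created up front but not displayed by this graph.
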(event `self.ReceiveBeginPlay`
  ;[1 1 1] Create the start game HUD widget
  (bind _returnvalue (`|CreateWidget` "/Game/HUDWidgets/WG_StartGameHUD.WG_StartGameHUD_C" (`GameplayStatics.GetPlayerController` 0)))
  (bind _output_get (set `self.StartGameHUD` _returnvalue))
  (`/Game/HUDWidgets/WG_StartGameHUD.ShowHUD` _output_get)
  ;[1 1 1] Create the Main Game HUD Widget
  (bind _returnvalue_2 (`|CreateWidget` "/Game/HUDWidgets/WG_MainGameHUD.WG_MainGameHUD_C" (`GameplayStatics.GetPlayerController` 0)))
  (set `self.MainGameHUD` _returnvalue_2)
  ;[1 1 1] Create the game over HUD widget
  (bind _returnvalue_3 (`|CreateWidget` "/Game/HUDWidgets/WG_GameOverHUD.WG_GameOverHUD_C" (`GameplayStatics.GetPlayerController` 0)))
  (set `self.GameOverHUD` _returnvalue_3)
  ;[1 1 1] Create the pause HUD widget
  (bind _returnvalue_4 (`|CreateWidget` "/Game/HUDWidgets/WG_PauseHUD.WG_PauseHUD_C" (`GameplayStatics.GetPlayerController` 0)))
  (set `self.PauseHUD` _returnvalue_4))

(fn `UserConstructionScript`)