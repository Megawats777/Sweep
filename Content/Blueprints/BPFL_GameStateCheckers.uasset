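; Blueprint function library of predicates that test a game state enum value.
; Separate functions report whether the passed-in state is starting, active, paused or finished.
; Each is a single equality comparison against one enumerator and reads nothing beyond its argument, so the caller supplies the current state.
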(fn `isGameActive`
  (params (CurrentGameState :type "/Game/Blueprints/Enumerations/GameStates Enum"))
  (returns (Result :type Boolean))
  (return (`|EnumEquality` CurrentGameState "NewEnumerator1")))

(fn `isGameFinished`
  (params (CurrentGameState :type "/Game/Blueprints/Enumerations/GameStates Enum"))
  (returns (Result :type Boolean))
  (return (`|EnumEquality` CurrentGameState "NewEnumerator3")))

(fn `isGamePaused`
  (params (CurrentGameState :type "/Game/Blueprints/Enumerations/GameStates Enum"))
  (returns (Result :type Boolean))
  (return (`|EnumEquality` CurrentGameState "NewEnumerator2")))

(fn `isGameStarting`
  (params (CurrentGameState :type "/Game/Blueprints/Enumerations/GameStates Enum"))
  (returns (Result :type Boolean))
  (return (`|EnumEquality` CurrentGameState "NewEnumerator0")))